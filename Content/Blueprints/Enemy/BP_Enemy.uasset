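; BP_Enemy is an enemy character with a cube mesh that dissolves away when killed.
; Destroy plays a plop sound, turns off the cube's collision, deactivates character movement and sets the Destroyed flag.
; While that flag is set, Tick raises the material's Progress parameter over about a quarter second, then destroys the actor.
; An AIMoveTo node is left unconnected, so this graph drives no movement.
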(event `self.ReceiveTick`
  (params (DeltaSeconds :type "Float (single-precision)"))
  (if (`self.Destroyed`)
    (bind _output_get (set `self.DissolveProgress` (+ (* DeltaSeconds 4.0) (`self.DissolveProgress`))))
    (`MeshComponent.SetScalarParameterValueOnMaterials` (`self.Cube`) "Progress" _output_get)
    (if (> _output_get 1.0)
      (`self.K2_DestroyActor`))))

(fn `Destroy`
  (`GameplayStatics.PlaySoundAtLocation` "/Game/Assets/Audio/SFX/Enemy/Plop.Plop" (`self.K2_GetActorLocation`) (struct) 1.0 1.0 0.0 null null null null)
  (set `self.Destroyed` true)
  (`PrimitiveComponent.SetCollisionEnabled` (`self.Cube`) "NoCollision")
  (`ActorComponent.Deactivate` (`self.CharacterMovement`)))

(fn `UserConstructionScript`)