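; Player pawn Blueprint for a mouse-aimed, twin-stick style control scheme.
; On BeginPlay it adds the Main_IMC Enhanced Input mapping context through Main_PlayerController.
; Each tick it deprojects the mouse cursor, line-traces against static and dynamic world objects, and yaws the actor toward the hit point.
; Move_IA drives movement input along fixed world X and Y axes, independent of facing.
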(event `self.ReceiveBeginPlay`
  (bind _asmain_player_controller (cast `/Game/Blueprints/Player/Main_PlayerController` (`GameplayStatics.GetPlayerController` 0)))
  (`EnhancedInputSubsystemInterface.AddMappingContext` (pcsubsystem `EnhancedInputLocalPlayerSubsystem` _asmain_player_controller) "/Game/Input/Main_IMC.Main_IMC" 0 (struct)))

(event `self.ReceiveTick`
  (params (DeltaSeconds :type "Float (single-precision)"))
  (bind _returnvalue_location (`KismetMathLibrary.BreakTransform` (`self.GetTransform`)))
  (bind _asmain_player_controller (cast `/Game/Blueprints/Player/Main_PlayerController` (`self.GetController`)))
  (bind (_worldlocation _worlddirection) (`PlayerController.DeprojectMousePositionToWorld` _asmain_player_controller))
  (bind (_outhit _returnvalue) (`KismetSystemLibrary.LineTraceSingleForObjects` _worldlocation (+ _worldlocation (* _worlddirection 10000.0)) (`|MakeArray` "ObjectTypeQuery1" "ObjectTypeQuery2" :!type "EObjectTypeQuery Enum")))
  (if _returnvalue
    (bind (_returnvalue_roll _returnvalue_pitch _returnvalue_yaw) (`KismetMathLibrary.BreakRotator` (`KismetMathLibrary.FindLookAtRotation` _returnvalue_location (`.ImpactPoint` (`GameplayStatics.BreakHitResult` _outhit)))))
    (`self.K2_SetActorRotation` (`KismetMathLibrary.MakeRotator` 0.0 0.0 _returnvalue_yaw))))

(event `EnhancedInput|/Game/Input/Move_IA`
  (params (ActionValue :type "Vector2D Structure") (ElapsedSeconds :type "Float (double-precision)") (TriggeredSeconds :type "Float (double-precision)") (InputAction :type "InputAction Object Reference" :default "/Game/Input/Move_IA.Move_IA"))
  (:`Triggered`
    (`self.AddMovementInput` (1.0 0.0 0.0) ActionValue_X)
    (`self.AddMovementInput` (0.0 1.0 0.0) ActionValue_Y)))

(fn `UserConstructionScript`)